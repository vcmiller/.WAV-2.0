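; Base character Blueprint providing health, weapon switching, combo attacks, dodge rolls, forward jumps and pivot turning.
; Attack, roll and jump use request flags and separate start/stop functions, with combo phases cycling through the current weapon's attacks until a timeout resets them.
; BP_Weapon child actors register into a weapon array that handles activation and damage windows.
; Rolling hides the weapon and blocks damage; depleted health calls an empty OnDeath hook.
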(event `self.ReceiveBeginPlay`
  (set `self.Health` (`self.MaxHealth`)))

(event `self.ReceiveAnyDamage`
  (params (Damage :type "Float (single-precision)") (DamageType :type "DamageType Object Reference") (InstigatedBy :type "Controller Object Reference") (DamageCauser :type "Actor Object Reference"))
  (if (not (`self.HasRollInvin`))
    (bind _output_get (set `self.Health` (- (`self.Health`) Damage)))
    (`/Engine/EditorBlueprintResources/StandardMacros.CompareFloat` _output_get
      (:`==`
        _)
      (:`<`
        _))
    (`self.OnDeath`)))

(fn `AddWeaponFromChildActor`
  (params (Component :type "ChildActorComponent Object Reference"))
  (returns (WeaponObject :type "/Game/Blueprints/Weapons/BP_Weapon Object Reference"))
  (bind _asbp_weapon (cast `/Game/Blueprints/Weapons/BP_Weapon` (`ChildActorComponent.ChildActor` Component))
    (:`then`
      (`KismetArrayLibrary.Array_AddUnique` (`self.Weapons`) _asbp_weapon)
      (return _asbp_weapon))
    (:`CastFailed`
      (return null))))

(fn `BeginAttack`
  (set `self.WantsToAttack` false)
  (`self.SetActiveWeapon` (`self.DesiredWeapon`))
  (set `self.LastAttackTime` (`KismetSystemLibrary.GetGameTimeInSeconds`)))

(fn `GetCurAttackAnim`
  (returns (Out :type "AnimSequenceBase Object Reference"))
  (return (`KismetArrayLibrary.Array_Get` (`/Game/Blueprints/Weapons/BP_Weapon.Attacks` (`KismetArrayLibrary.Array_Get` (`self.Weapons`) (`self.DesiredWeapon`))) (`self.AttackPhase`))))

(fn `GetCurWeapon`
  (returns (Out :type "/Game/Blueprints/Weapons/BP_Weapon Object Reference"))
  (return (`KismetArrayLibrary.Array_Get` (`self.Weapons`) (`self.Weapon`))))

(fn `JumpActivate`
  (bind (_returnvalue_x _returnvalue_y) (`KismetMathLibrary.BreakVector` (* (`self.GetActorForwardVector`) (`self.JumpSpeedForward`))))
  (set `self.WantsToJump` false)
  (`self.LaunchCharacter` (`KismetMathLibrary.MakeVector` _returnvalue_x _returnvalue_y (`self.JumpSpeedUp`)))
  (set `self.Jumping` true))

(fn `JumpLand`
  (set `self.Jumping` false))

(fn `OnDeath`)

(fn `PivotEnd`
  (set `self.Pivoting` false))

(fn `PivotStart`
  (set `self.Pivoting` true))

(fn `PivotTowards`
  (params (TargetDir :type "Vector Structure"))
  (`self.K2_SetActorRotation` (`KismetMathLibrary.RInterpTo` (`self.K2_GetActorRotation`) (`KismetMathLibrary.MakeRotFromZX` (0.0 0.0 1.0) TargetDir) (`GameplayStatics.GetWorldDeltaSeconds`) (`self.PivotRate`))))

(fn `QueueAttack`
  (params (Phase :type Integer) (Weapon :type Integer))
  (if (`KismetMathLibrary.BooleanNOR` (`NavMovementComponent.IsFalling` (`self.CharacterMovement`)) (`self.WantsToAttack`))
    (set `self.DesiredWeapon` Weapon)
    (set `self.AttackPhase` Phase)
    (set `self.WantsToAttack` true)))

(fn `QueueNextAttack`
  (params (Weapon :type Integer))
  (`self.QueueAttack` (select `bool` (> (- (`KismetSystemLibrary.GetGameTimeInSeconds`) (`self.LastAttackTime`)) (`/Game/Blueprints/Weapons/BP_Weapon.PhaseReset` (`self.GetCurWeapon`))) :`false` (mod (+ (`self.AttackPhase`) 1) (`KismetArrayLibrary.Array_Length` (`/Game/Blueprints/Weapons/BP_Weapon.Attacks` (`self.GetCurWeapon`))))) Weapon))

(fn `QueueRoll`
  (if (> (- (`KismetSystemLibrary.GetGameTimeInSeconds`) (`self.LastRollTime`)) (`self.RollCooldown`))
    (set `self.WantsToRoll` true)))

(fn `SetActiveWeapon`
  (params (Index :type Integer))
  (bind _weapons (`self.Weapons`))
  (bind _weapon (`self.Weapon`))
  (if (!= Index _weapon)
    (`/Game/Blueprints/Weapons/BP_Weapon.SetActive` (`KismetArrayLibrary.Array_Get` _weapons _weapon) false)
    (bind _output_get (set `self.Weapon` Index))
    (`/Game/Blueprints/Weapons/BP_Weapon.SetActive` (`KismetArrayLibrary.Array_Get` _weapons _output_get) true)
    (else
      (return))))

(fn `StartDamage`
  (`/Game/Blueprints/Weapons/BP_Weapon.StartDamage` (`self.GetCurWeapon`)))

(fn `StartRoll`
  (`/Game/Blueprints/Weapons/BP_Weapon.SetActive` (`self.GetCurWeapon`) false)
  (set `self.HasRollInvin` true))

(fn `StopDamage`
  (`/Game/Blueprints/Weapons/BP_Weapon.EndDamage` (`self.GetCurWeapon`))
  (set `self.Attacking` false))

(fn `StopRoll`
  (set `self.WantsToRoll` false)
  (`/Game/Blueprints/Weapons/BP_Weapon.SetActive` (`self.GetCurWeapon`) true)
  (set `self.HasRollInvin` false)
  (set `self.LastRollTime` (`KismetSystemLibrary.GetGameTimeInSeconds`)))

(fn `UserConstructionScript`)