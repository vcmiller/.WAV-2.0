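; Player character with zone-based cameras, camera-relative movement and three melee attack inputs.
; Overlapped BP_CamZone cameras form a list, and Tick blends the view to the newest.
; Grounded attack inputs queue a weapon and alternate a two-step AttackPhase that resets on a timer; BeginAttack swaps the weapon mesh, whose overlaps apply damage.
; While attacking, movement and jump input are ignored, and input steers facing at a capped turn rate.
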(event `self.ReceiveTick`
  (params (DeltaSeconds :type "Float (single-precision)"))
  (`self.CameraControl`
    (:`One Comes Out`
      (`self.UpdateRotation`)
      (bind _output_get (set `self.TimeUntilPhaseReset` (- (`self.TimeUntilPhaseReset`) DeltaSeconds)))
      (if (and (< _output_get 0.0) (not (`self.WantsToAttack`)))
        (set `self.AttackPhase` -1)))))

(event `self.ReceiveActorBeginOverlap`
  (params (OtherActor :type "Actor Object Reference"))
  ;[1 1 1] On Entering a New Camera Zone
  (bind _asbp_cam_zone (cast `/Game/Blueprints/BP_CamZone` OtherActor))
  (`KismetArrayLibrary.Array_AddUnique` (`self.CameraList`) (`/Game/Blueprints/BP_CamZone.CamActor` _asbp_cam_zone)))

(event `self.ReceiveActorEndOverlap`
  (params (OtherActor :type "Actor Object Reference"))
  ;[1 1 1] On Exiting a Camera Zone
  (bind _asbp_cam_zone (cast `/Game/Blueprints/BP_CamZone` OtherActor))
  (`KismetArrayLibrary.Array_RemoveItem` (`self.CameraList`) (`/Game/Blueprints/BP_CamZone.CamActor` _asbp_cam_zone)))

(event `self.ReceiveBeginPlay`
  (`PlayerController.SetViewTargetWithBlend` (`GameplayStatics.GetPlayerController` 0) (`KismetArrayLibrary.Array_Get` (`self.CameraList`)) 0.0 "VTBlend_Linear" 0.0 false))

(event `InputAction|Jump`
  (params (Key :type "Key Structure" :default "AnyKey"))
  (:`Pressed`
    (if (not (`self.Attacking`))
      (`self.Jump`)))
  (:`Released`
    (`self.StopJumping`)))

(event `InputAxis|MoveForward`
  (params (AxisValue :type "Float (single-precision)"))
  (bind (_returnvalue_x _returnvalue_y) (`KismetMathLibrary.BreakVector` (`self.GetActorForwardVector` (`Controller.GetViewTarget` (`GameplayStatics.GetPlayerController` 0)))))
  (if (not (`self.Attacking`))
    (`self.AddMovementInput` (`KismetMathLibrary.Normal` (`KismetMathLibrary.MakeVector` _returnvalue_x _returnvalue_y)) AxisValue)))

(event `InputAxis|MoveRight`
  (params (AxisValue :type "Float (single-precision)"))
  (bind (_returnvalue_x _returnvalue_y) (`KismetMathLibrary.BreakVector` (`self.GetActorRightVector` (`Controller.GetViewTarget` (`GameplayStatics.GetPlayerController` 0)))))
  (if (not (`self.Attacking`))
    (`self.AddMovementInput` (`KismetMathLibrary.Normal` (`KismetMathLibrary.MakeVector` _returnvalue_x _returnvalue_y)) AxisValue)))

(event `InputAction|Attack1`
  (params (Key :type "Key Structure" :default "AnyKey"))
  ;[1 1 1] Attacks
  (:`Pressed`
    (`self.AttackInput` 0)))

(event `InputAction|Attack2`
  (params (Key :type "Key Structure" :default "AnyKey"))
  ;[1 1 1] Attacks
  (:`Pressed`
    (`self.AttackInput` 1)))

(event `InputAction|Attack3`
  (params (Key :type "Key Structure" :default "AnyKey"))
  ;[1 1 1] Attacks
  (:`Pressed`
    (`self.AttackInput` 2)))

(event `self.WeaponMesh.OnComponentBeginOverlap`
  (params (OverlappedComponent :type "PrimitiveComponent Object Reference") (OtherActor :type "Actor Object Reference") (OtherComp :type "PrimitiveComponent Object Reference") (OtherBodyIndex :type Integer) (bFromSweep :type Boolean) (SweepResult :type "HitResult Structure (by ref)"))
  (`GameplayStatics.ApplyDamage` OtherActor (`self.WeaponDamage`)))

(fn `AttackInput`
  (params (Weapon :type Integer))
  (if (`KismetMathLibrary.BooleanNOR` (`NavMovementComponent.IsFalling` (`self.CharacterMovement`)) (`self.WantsToAttack`))
    (set `self.WantsToAttack` true)
    (set `self.Weapon` Weapon)
    (set `self.AttackPhase` (mod (+ (`self.AttackPhase`) 1) 2))))

(fn `BeginAttack`
  (params (Weapon :type Integer))
  (bind _weaponmesh (`self.WeaponMesh`))
  (bind _item (`KismetArrayLibrary.Array_Get` (`self.WeaponScales`) Weapon))
  (set `self.Attacking` true)
  (set `self.WantsToAttack` false)
  (set `self.TimeUntilPhaseReset` (`KismetArrayLibrary.Array_Get` (`self.AttackPhaseReset`) Weapon))
  (`StaticMeshComponent.SetStaticMesh` _weaponmesh (`KismetArrayLibrary.Array_Get` (`self.WeaponMeshes`) Weapon))
  (`SceneComponent.SetRelativeScale3D` _weaponmesh (`KismetMathLibrary.MakeVector` _item _item _item))
  (if (!= (`self.PrevWeapon`) Weapon)
    (`ActorComponent.Activate` (`self.WeaponParticles`) false)
    (set `self.PrevWeapon` Weapon)))

(fn `RotationDuringAttack`
  (bind _returnvalue (`self.GetActorForwardVector`))
  (bind (_returnvalue_roll _returnvalue_pitch _returnvalue_yaw) (`KismetMathLibrary.BreakRotator` (`self.K2_GetActorRotation`)))
  (bind _returnvalue_2 (`Controller.GetViewTarget` (`GameplayStatics.GetPlayerController` 0)))
  (bind (_returnvalue_x _returnvalue_y) (`KismetMathLibrary.BreakVector` (`self.GetActorForwardVector` _returnvalue_2)))
  (bind (_returnvalue_x_2 _returnvalue_y_2) (`KismetMathLibrary.BreakVector` (`self.GetActorRightVector` _returnvalue_2)))
  (bind _returnvalue_3 (`KismetMathLibrary.Normal` (+ (* (`KismetMathLibrary.Normal` (`KismetMathLibrary.MakeVector` _returnvalue_x _returnvalue_y)) (`self.GetInputAxisValue`)) (* (`KismetMathLibrary.Normal` (`KismetMathLibrary.MakeVector` _returnvalue_x_2 _returnvalue_y_2)) (`self.GetInputAxisValue`)))))
  (bind (_returnvalue_x_3 _returnvalue_y_3 _returnvalue_z) (`KismetMathLibrary.BreakVector` (`KismetMathLibrary.Cross_VectorVector` _returnvalue _returnvalue_3)))
  (`self.K2_SetActorRotation` (`KismetMathLibrary.MakeRotator` _returnvalue_roll _returnvalue_pitch (+ (* (`KismetMathLibrary.FClamp` (`KismetMathLibrary.DegAcos` (`KismetMathLibrary.Dot_VectorVector` _returnvalue _returnvalue_3)) 0.0 (* (`self.RotateSpeedAttacking`) (`GameplayStatics.GetWorldDeltaSeconds`))) (`KismetMathLibrary.SignOfFloat` _returnvalue_z)) _returnvalue_yaw))))

(fn `UpdateRotation`
  (bind _attacking (`self.Attacking`))
  (set `CharacterMovementComponent.bOrientRotationToMovement` (not _attacking) (`self.CharacterMovement`))
  (if _attacking
    (`self.RotationDuringAttack`)))

(fn `UserConstructionScript`)