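; Base-style melee weapon Blueprint that applies damage to overlapping actors during an active swing window and shows a sword trail.
; StartDamage clears the per-swing hit list and starts the BP_SwordTrail child actor's sweep, while EndDamage closes the window.
; Overlaps damage each new actor and play a random hit sound, unless a NoHitClasses entry is a child of its class.
; SetActive toggles mesh visibility and collision.
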(event `self.ReceiveBeginPlay`
  (bind _asbp_sword_trail (cast `/Game/Blueprints/Weapons/BP_SwordTrail` (`ChildActorComponent.ChildActor` (`self.Trail`))))
  (set `self.TrailObject` _asbp_sword_trail))

(event `self.ReceiveActorBeginOverlap`
  (params (OtherActor :type "Actor Object Reference"))
  (`self.OnHitObject` OtherActor))

(fn `EndDamage`
  (set `self.DamageActive` false)
  (`SceneComponent.SetVisibility` (`self.Trail`) false false))

(fn `OnHitObject`
  (params (HitActor :type "Actor Object Reference"))
  (returns (Damaged :type Boolean))
  (locals (FoundClass :type Boolean))
  (bind _hitsounds (`self.HitSounds`))
  (bind _returnvalue (`BlueprintSetLibrary.Set_Add` (`self.HitThisSwing`) HitActor))
  (if (and _returnvalue (`self.DamageActive`))
    (for _array_element (`self.NoHitClasses`)
      (if (`KismetMathLibrary.ClassIsChildOf` _array_element (`GameplayStatics.GetObjectClass` HitActor))
        (set `local.FoundClass` true)))
    (if (`local.FoundClass`)
      (return false)
      (else
        (`GameplayStatics.ApplyDamage` HitActor (`self.Damage`) null self)
        (if (> (`KismetArrayLibrary.Array_Length` _hitsounds) 0)
          (`GameplayStatics.PlaySoundAtLocation` (`KismetArrayLibrary.Array_Get` _hitsounds (`KismetMathLibrary.RandomInteger` (`KismetArrayLibrary.Array_Length` _hitsounds))) (`self.K2_GetActorLocation`) (struct) 1.0 1.0 0.0 "/Game/Audio/IDKWhyIHaveToMakeThis.IDKWhyIHaveToMakeThis"))
        (return true)))
    (else
      (return false))))

(fn `SetActive`
  (params (`Active?` :type Boolean))
  (bind _staticmesh (`self.StaticMesh`))
  (`SceneComponent.SetVisibility` _staticmesh `Active?` false)
  (`PrimitiveComponent.SetCollisionEnabled` _staticmesh (select `bool` `Active?` :`false` "NoCollision" :`true` "QueryAndPhysics" :!type "ECollisionEnabled Enum"))
  (if (not `Active?`)
    (`self.EndDamage`)))

(fn `StartDamage`
  (`BlueprintSetLibrary.Set_Clear` (`self.HitThisSwing`))
  (set `self.DamageActive` true)
  (`/Game/Blueprints/Weapons/BP_SwordTrail.BeginSweep` (`self.TrailObject`))
  (`SceneComponent.SetVisibility` (`self.Trail`) true false))

(fn `UserConstructionScript`)