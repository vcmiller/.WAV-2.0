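; BP_SwordTrail draws a sword swing trail as a procedural mesh strip built from two local edge points.
; BeginPlay builds triangles and UVs; while enabled, Tick shifts the world-space vertex history and rebuilds the mesh in local space.
; UpdatePreviousP smooths fast motion by interpolating transforms between the previous and current frame.
; BeginSweep collapses the history onto Vertex1 at the current transform, since its `Index % 1` select never picks Vertex2.
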(event `self.ReceiveTick`
  (params (DeltaSeconds :type "Float (single-precision)"))
  (`SceneComponent.SetVisibility` (`self.Trail`) (`self.Enabled`) false)
  (if (`self.Enabled`)
    (`self.UpdatePreviousP`)
    (`ProceduralMeshComponent.CreateMeshSection_LinearColor` :`self` (`self.Trail`) :`Vertices` (`self.MapVertexArray`) :`Triangles` (`self.Triangles`) :`UV0` (`self.UVs`))
    (`PrimitiveComponent.SetMaterial` (`self.Trail`) 0 (`self.Material`))))

(event `self.ReceiveBeginPlay`
  (bind _triangles (`self.Triangles`))
  (bind _returnvalue (* (`self.FrameCount`) (`self.InterpCount`)))
  (bind _returnvalue_2 (- _returnvalue 1))
  (for _index (range (+ (- _returnvalue 2) 1))
    (`KismetArrayLibrary.Array_Add` _triangles (+ _index 0))
    (`KismetArrayLibrary.Array_Add` _triangles (+ _index 1))
    (`KismetArrayLibrary.Array_Add` _triangles (+ _index 2)))
  (for _ (range (+ _returnvalue_2 1))
    (`KismetArrayLibrary.Array_Add` (`self.Vertices`) (0.0 0.0 0.0)))
  (for _index_2 (range (+ _returnvalue_2 1))
    (`KismetArrayLibrary.Array_Add` (`self.UVs`) (`KismetMathLibrary.MakeVector2D` (/ (`KismetMathLibrary.Conv_IntToDouble` (/ _index_2 2)) (/ (`KismetMathLibrary.Conv_IntToDouble` (* (`self.FrameCount`) (`self.InterpCount`))) 2.0)) (- 1.0 (`KismetMathLibrary.Conv_IntToDouble` (mod _index_2 2))))))
  (`ProceduralMeshComponent.CreateMeshSection_LinearColor` :`self` (`self.Trail`) :`Vertices` (`self.Vertices`) :`Triangles` (`self.Triangles`) :`UV0` (`self.UVs`) :`bCreateCollision` true)
  (set `self.Generated` true)
  (`self.UpdatePreviousP`)
  (`PrimitiveComponent.SetMaterial` (`self.Trail`) 0 "/Game/Materials/M_SwordTrailRed.M_SwordTrailRed"))

(fn `BeginSweep`
  (bind _returnvalue (`self.GetTransform`))
  (for _index (range (+ (`KismetArrayLibrary.Array_LastIndex` (`self.Vertices`)) 1))
    (`KismetArrayLibrary.Array_Set` (`self.Vertices`) _index (`KismetMathLibrary.TransformLocation` _returnvalue (select `int` (mod _index 1) :`0` (`self.Vertex1`) :`1` (`self.Vertex2`))))
    (set `self.PrevT` _returnvalue)))

(fn `MapVertexArray`
  (returns (Out :type "Array of Vector Structure"))
  (bind _tempvertices (`self.TempVertices`))
  (`KismetArrayLibrary.Array_Clear` (`self.TempVertices`))
  (for _array_element (`self.Vertices`)
    (`KismetArrayLibrary.Array_Add` _tempvertices (`KismetMathLibrary.InverseTransformLocation` (`self.GetTransform`) _array_element)))
  (return _tempvertices))

(fn `UpdatePreviousP`
  (bind _vertices (`self.Vertices`))
  (bind _vertices_2 (`self.Vertices`))
  (bind _returnvalue (`KismetArrayLibrary.Array_LastIndex` (`self.Vertices`)))
  (set `self.CurT` (`self.GetTransform`))
  (for _index (range (+ (- _returnvalue (* (`self.InterpCount`) 2)) 1))
    (bind _returnvalue_2 (- _returnvalue _index))
    (`KismetArrayLibrary.Array_Set` _vertices_2 _returnvalue_2 (`KismetArrayLibrary.Array_Get` _vertices_2 (- _returnvalue_2 (* (`self.InterpCount`) 2)))))
  (for _index_2 (range (`self.InterpCount`))
    (bind _returnvalue_3 (* _index_2 2))
    (bind _returnvalue_4 (/ (`KismetMathLibrary.Conv_IntToDouble` (+ _index_2 1)) (`KismetMathLibrary.Conv_IntToDouble` (`self.InterpCount`))))
    (`KismetArrayLibrary.Array_Set` _vertices _returnvalue_3 (`KismetMathLibrary.TransformLocation` (`KismetMathLibrary.TLerp` (`self.CurT`) (`self.PrevT`) _returnvalue_4) (`self.Vertex1`)))
    (`KismetArrayLibrary.Array_Set` _vertices (+ _returnvalue_3 1) (`KismetMathLibrary.TransformLocation` (`KismetMathLibrary.TLerp` (`self.CurT`) (`self.PrevT`) _returnvalue_4) (`self.Vertex2`))))
  (set `self.PrevT` (`self.CurT`)))

(fn `UserConstructionScript`)