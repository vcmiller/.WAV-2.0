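; Base Blueprint for player weapons that caches its owning BP_Player on BeginPlay and resolves which upgrades are equipped.
; The upgrade getters look up two slot keys in the player's ItemSlots map and return the item with an Equipped flag.
; Primary falls back from slot 1 to slot 2, while secondary reports slot 2 only when both are filled.
; UpdateWeapon is an empty function here.
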(event `self.ReceiveBeginPlay`
  (`parent.ReceiveBeginPlay`)
  (bind _asbp_player (cast `/Game/Blueprints/Player/BP_Player` (`self.GetOwner`)))
  (set `self.Player` _asbp_player))

(fn `GetPrimaryUpgrade`
  (returns (Item :type Integer) (Equipped :type Boolean))
  (bind _itemslots (`/Game/Blueprints/Player/BP_Player.ItemSlots` (`self.Player`)))
  (bind (_value _returnvalue) (`BlueprintMapLibrary.Map_Find` _itemslots (`self.UpgradeSlot1`)))
  (bind (_value_2 _returnvalue_2) (`BlueprintMapLibrary.Map_Find` _itemslots (`self.UpgradeSlot2`)))
  (if _returnvalue
    (return _value true)
    (elif _returnvalue_2
      (return _value_2 true)
      (else
        (return -1 false)))))

(fn `GetSecondaryUpgrade`
  (returns (Item :type Integer) (Equipped :type Boolean))
  (bind _itemslots (`/Game/Blueprints/Player/BP_Player.ItemSlots` (`self.Player`)))
  (bind (_value _returnvalue) (`BlueprintMapLibrary.Map_Find` _itemslots (`self.UpgradeSlot2`)))
  (if (`.ReturnValue` (`BlueprintMapLibrary.Map_Find` _itemslots (`self.UpgradeSlot1`)))
    (if _returnvalue
      (return _value true)
      (else
        (return -1 false)))
    (else
      (return -1 false))))

(fn `UpdateWeapon`)

(fn `UserConstructionScript`
  (`parent.UserConstructionScript`))