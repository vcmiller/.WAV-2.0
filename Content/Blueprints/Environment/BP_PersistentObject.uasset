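; BP_PersistentObject is a base Blueprint for environment objects whose state persists in a save game.
; Load caches the SaveInstance, looks up the object's name in its PersistantObjectStates map, and on a match restores State and calls the empty OnLoad hook.
; SetState calls Save only when the value changes, which updates the map entry, writes the slot immediately and prints the result and slot name.
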(event `Load`
  (params (SaveInstance :type "/Game/Blueprints/Player/BP_Save Object Reference"))
  (bind _output_get (set `self.SaveInstance` SaveInstance))
  (bind (_value _returnvalue) (`BlueprintMapLibrary.Map_Find` (`/Game/Blueprints/Player/BP_Save.PersistantObjectStates` _output_get) (`KismetSystemLibrary.GetObjectName` self)))
  (if _returnvalue
    (set `self.State` _value)
    (`self.OnLoad`)))

(event `Save`
  (bind _saveinstance (`self.SaveInstance`))
  (bind _slotname (`/Game/Blueprints/Player/BP_Save.SlotName` _saveinstance))
  (`BlueprintMapLibrary.Map_Add` (`/Game/Blueprints/Player/BP_Save.PersistantObjectStates` (`self.SaveInstance`)) (`KismetSystemLibrary.GetObjectName` self) (`self.State`))
  (bind _returnvalue (`GameplayStatics.SaveGameToSlot` _saveinstance _slotname (`/Game/Blueprints/Player/BP_Save.UserIndex` _saveinstance)))
  (`KismetSystemLibrary.PrintString` (`KismetStringLibrary.Conv_BoolToString` _returnvalue))
  (`KismetSystemLibrary.PrintString` _slotname))

(fn `GetState`
  (returns (State :type Integer))
  (return (`self.State`)))

(fn `OnLoad`)

(fn `SetState`
  (params (NewState :type Integer))
  (if (!= NewState (`self.State`))
    (set `self.State` NewState)
    (`self.Save`)))

(fn `UserConstructionScript`)