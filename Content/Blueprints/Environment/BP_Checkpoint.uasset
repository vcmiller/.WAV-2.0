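; Checkpoint actor that becomes the single active checkpoint when BP_Player overlaps its trigger.
; Activation finds the current one by scanning all BP_Checkpoint actors for state 1, switches it off, then turns itself on.
; An integer state, accessed through GetState and SetState, drives the cylinder's visibility and the particle system, and OnLoad reapplies both from that state.
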(event `self.OnLoad`
  (bind _state (`self.GetState`))
  (bind _returnvalue (`KismetMathLibrary.Conv_IntToBool` _state))
  (`SceneComponent.SetVisibility` (`self.Cylinder`) _returnvalue false)
  (`ActorComponent.SetActive` (`self.ParticleSystem`) _returnvalue false))

(event `self.Trigger.OnComponentBeginOverlap`
  (params (OverlappedComponent :type "PrimitiveComponent Object Reference") (OtherActor :type "Actor Object Reference") (OtherComp :type "PrimitiveComponent Object Reference") (OtherBodyIndex :type Integer) (bFromSweep :type Boolean) (SweepResult :type "HitResult Structure (by ref)"))
  (cast `/Game/Blueprints/BP_Player` OtherActor)
  (`self.Activate`))

(fn `Activate`
  (bind _state (`self.GetState`))
  (if (== _state 0)
    (bind _out (`self.GetCurrentCheckpoint`))
    (`/Engine/EditorBlueprintResources/StandardMacros.IsValid` _out
      (:`Is Valid`
        (`self.SetActive` _out false))
      (:`Is Not Valid`
        _))
    (`self.SetActive` true)))

(fn `GetCurrentCheckpoint`
  (returns (Out :type "/Game/Blueprints/Environment/BP_Checkpoint Object Reference"))
  (bind _outactors (`GameplayStatics.GetAllActorsOfClass` "BP_Checkpoint_C"))
  (for _array_element _outactors
    (bind _state (`self.GetState` _array_element))
    (if (== _state 1)
      (return _array_element)))
  (return null))

(fn `SetActive`
  (params (`Active?` :type Boolean))
  (locals (Active :type Boolean))
  (bind _output_get (set `local.Active` `Active?`))
  (bind _state (`self.GetState`))
  (bind _returnvalue (`KismetMathLibrary.Conv_BoolToInt` _output_get))
  (if (!= _state _returnvalue)
    (`self.SetState` _returnvalue)
    (`SceneComponent.SetVisibility` (`self.Cylinder`) (`local.Active`) false)
    (`ActorComponent.SetActive` (`self.ParticleSystem`) (`local.Active`) false)
    (`self.SetState` (`KismetMathLibrary.Conv_BoolToInt` (`local.Active`)))))

(fn `UserConstructionScript`)