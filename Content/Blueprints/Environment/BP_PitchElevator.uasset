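; BP_PitchElevator is an environment elevator actor whose materials brighten once its glow is active.
; BeginPlay creates dynamic material instances for the Elevator and Glow components and applies the starting Brightness to both.
; While GlowActive is set, Tick raises or lowers Brightness at a constant rate toward a fixed target and pushes it to both materials through UpdateMaterials.
; The graph contains no movement logic and never sets GlowActive itself.
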(event `self.ReceiveBeginPlay`
  (bind _returnvalue (`PrimitiveComponent.CreateDynamicMaterialInstance` (`self.Elevator`) 0 null))
  (set `self.ElevatorMat` _returnvalue)
  (bind _returnvalue_2 (`PrimitiveComponent.CreateDynamicMaterialInstance` (`self.Glow`) 0 null))
  (set `self.GlowMat` _returnvalue_2)
  (`self.UpdateMaterials`))

(event `self.ReceiveTick`
  (params (DeltaSeconds :type "Float (single-precision)"))
  (if (`self.GlowActive`)
    (set `self.Brightness` (`KismetMathLibrary.FInterpTo_Constant` (`self.Brightness`) 2.0 DeltaSeconds 0.5))
    (`self.UpdateMaterials`)))

(event `UpdateMaterials`
  (`MaterialInstanceDynamic.SetScalarParameterValue` (`self.ElevatorMat`) "Brightness" (`self.Brightness`))
  (`MaterialInstanceDynamic.SetScalarParameterValue` (`self.GlowMat`) "Brightness" (`self.Brightness`)))

(fn `UserConstructionScript`)