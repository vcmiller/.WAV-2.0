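; Camera actor that follows the player along a camera rail by tracking the closest point on the rail's spline.
; On BeginPlay it takes the first BP_Player and casts the owner of its attach parent to CameraRig_Rail.
; Each Tick it finds the spline point nearest the player and moves most of the way there with a fixed-alpha lerp, so smoothing depends on frame rate.
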(event `self.ReceiveBeginPlay`
  (bind _outactors (`GameplayStatics.GetAllActorsOfClass` "/Game/Blueprints/Player/BP_Player.BP_Player_C"))
  (set `self.Player` (`KismetArrayLibrary.Array_Get` _outactors))
  (set `self.CameraSpline` (cast `CameraRig_Rail` (`ActorComponent.GetOwner` (`SceneComponent.GetAttachParent` (`self.K2_GetRootComponent`))) :!pure true)))

(event `self.ReceiveTick`
  (params (DeltaSeconds :type "Float (single-precision)"))
  (bind _returnvalue (`self.GetComponentByClass` (`self.CameraSpline`) "/Script/Engine.SplineComponent"))
  (`/Engine/EditorBlueprintResources/StandardMacros.IsValid` _returnvalue
    (:`Is Valid`
      (`self.K2_SetActorLocation` (`KismetMathLibrary.VLerp` (`SplineComponent.FindLocationClosestToWorldLocation` _returnvalue (`self.K2_GetActorLocation` (`self.Player`)) "World") (`self.K2_GetActorLocation`) 0.3)))))

(fn `UserConstructionScript`)