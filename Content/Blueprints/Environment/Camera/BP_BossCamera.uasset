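; Boss fight camera that keeps the boss in view while following behind the player.
; BeginPlay points look-at tracking at the Boss with a slight downward offset and excludes Player and Boss from traces.
; Each Tick line-traces against WorldStatic from the player toward a raised point back along the camera's forward axis.
; It lerps halfway to that point, or to just in front of any hit, using a swept move.
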(event `self.ReceiveBeginPlay`
  (bind _toignore (`self.ToIgnore`))
  (set `self.LookatTrackingSettings` (make `CameraLookatTrackingSettings` true false 50.0 (`self.Boss`) (0.0 0.0 -50.0)))
  (`KismetArrayLibrary.Array_AddUnique` _toignore (`self.Player`))
  (`KismetArrayLibrary.Array_AddUnique` _toignore (`self.Boss`)))

(event `self.ReceiveTick`
  (params (DeltaSeconds :type "Float (single-precision)"))
  (bind _returnvalue (`self.K2_GetActorLocation` (`self.Player`)))
  (bind _returnvalue_2 (`KismetMathLibrary.GetForwardVector` (`self.K2_GetActorRotation`)))
  (bind _returnvalue_3 (+ _returnvalue (0.0 0.0 150.0) (* _returnvalue_2 -1000.0)))
  (bind (_outhit _returnvalue_4) (`KismetSystemLibrary.LineTraceSingleForObjects` _returnvalue _returnvalue_3 (`|MakeArray` "ObjectTypeQuery1" :!type "EObjectTypeQuery Enum") false (`self.ToIgnore`)))
  (`self.K2_SetActorLocation` (`KismetMathLibrary.VLerp` (`self.K2_GetActorLocation`) (select `bool` _returnvalue_4 :`false` _returnvalue_3 :`true` (+ _returnvalue_2 (`.Location` (`GameplayStatics.BreakHitResult` _outhit)))) 0.5) true))

(fn `UserConstructionScript`)