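; BP_Waypoint is a path node actor that links to a successor through DefaultNext, exposed by GetNext.
; Its construction script flushes persistent debug lines, then has every BP_Waypoint in the world redraw its link, so the whole route refreshes whenever one is constructed.
; DrawLine draws a long-lasting blue debug line to a valid next waypoint.
; The event graph has no active logic.
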(fn `DrawLine`
  (bind _defaultnext (`self.DefaultNext`))
  (`/Engine/EditorBlueprintResources/StandardMacros.IsValid` _defaultnext
    (:`Is Valid`
      (`KismetSystemLibrary.DrawDebugLine` (`self.K2_GetActorLocation`) (`self.K2_GetActorLocation` _defaultnext) (struct :`G` 0.016063 :`B` 1.0 :`A` 1.0) 9999999999.0 5.0))))

(fn `GetNext`
  (returns (Next :type "/Game/Blueprints/Environment/BP_Waypoint Object Reference"))
  (return (`self.DefaultNext`)))

(fn `UserConstructionScript`
  (`KismetSystemLibrary.FlushPersistentDebugLines`)
  (bind _outactors (`GameplayStatics.GetAllActorsOfClass` "BP_Waypoint_C"))
  (for _array_element _outactors
    (`self.DrawLine` _array_element)))