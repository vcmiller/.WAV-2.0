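; BP_BossDoor is a boss door with a skeletal mesh that opens when BP_Player begins overlapping it.
; SetOpen acts only on a state change, playing DoorOpen or DoorClose once without looping.
; When closing, it also jumps the animation position to the play length of the Asdf animation, with notifies enabled, rather than playing from the start.
; Nothing in this Blueprint calls SetOpen to close the door.
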(event `SetOpen`
  (params (Open :type Boolean))
  (bind _skeletalmeshcomponent (`self.SkeletalMeshComponent`))
  (if (!= Open (`self.Open`))
    (bind _output_get (set `self.Open` Open))
    (`SkeletalMeshComponent.PlayAnimation` _skeletalmeshcomponent (select `bool` _output_get :`false` "/Game/Animation/Environment/DoorCLose.DoorClose" :`true` "/Game/Animation/Environment/DoorOpen.DoorOpen" :!type "AnimationAsset Object Reference") false)
    (if (not _output_get)
      (bind _returnvalue (`AnimSequenceBase.GetPlayLength` (`self.asdf`)))
      (`SkeletalMeshComponent.SetPosition` _skeletalmeshcomponent _returnvalue true))))

(event `self.ReceiveActorBeginOverlap`
  (params (OtherActor :type "Actor Object Reference"))
  (cast `/Game/Blueprints/Player/BP_Player` OtherActor)
  (`self.SetOpen` true))

(fn `UserConstructionScript`)