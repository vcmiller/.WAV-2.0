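; Boss enemy that fights the player with two fist weapons and thrown projectiles, and calls the player's end event when it dies.
; AttackPhase selects whether the right, left or both fists deal damage, and stopping damage disables both.
; BigThrow and SmallThrowSeries set a throw request flag.
; Projectiles spawn attached to a given component, then detach and launch as physics bodies aimed above the player's location.
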(event `self.OnDeath`
  (`parent.OnDeath`)
  (`/Game/Blueprints/Player/BP_Player.ENd` (`self.Player`)))

(event `self.ReceiveBeginPlay`
  (`parent.ReceiveBeginPlay`)
  (bind _weaponobject (`self.AddWeaponFromChildActor` (`self.FistR`)))
  (set `self.FistRWeapon` _weaponobject)
  (bind _weaponobject_2 (`self.AddWeaponFromChildActor` (`self.FistL`)))
  (set `self.FistLWeapon` _weaponobject_2))

(event `self.StartDamage`
  (switch `int` (`self.AttackPhase`)
    (:`0`
      (`/Game/Blueprints/Weapons/BP_Weapon.StartDamage` (`self.FistRWeapon`) :!label _label))
    (:`1`
      (`/Game/Blueprints/Weapons/BP_Weapon.StartDamage` (`self.FistLWeapon`) :!label _label_2))
    (:`2`
      (goto _label))
    (:`3`
      (`|ExecutionSequence`
        (:`then_0`
          (goto _label_2))
        (:`then_1`
          (goto _label))))))

(event `self.StopDamage`
  (`parent.StopDamage`)
  (`/Game/Blueprints/Weapons/BP_Weapon.EndDamage` (`self.FistLWeapon`))
  (`/Game/Blueprints/Weapons/BP_Weapon.EndDamage` (`self.FistRWeapon`)))

(fn `BigThrow`
  (set `self.WantsToThrow` 2))

(fn `LaunchProjectile`
  (bind _projectile (`self.Projectile`))
  (bind (_returnvalue_x _returnvalue_y _returnvalue_z) (`KismetMathLibrary.BreakVector` (`self.K2_GetActorLocation` (`self.Player`))))
  (bind _mesh (`/Game/Blueprints/Enemies/Projectiles/BP_Projectile_Base.Mesh` _projectile))
  (`/Engine/EditorBlueprintResources/StandardMacros.IsValid` (`self.Projectile`)
    (:`Is Valid`
      (`self.K2_DetachFromActor` (`self.Projectile`) "KeepWorld" "KeepWorld" "KeepWorld")
      (set `/Game/Blueprints/Enemies/Projectiles/BP_Projectile_Base.Thrown` true _projectile)
      (`PrimitiveComponent.SetSimulatePhysics` _mesh true)
      (`PrimitiveComponent.SetPhysicsLinearVelocity` _mesh (* (`KismetMathLibrary.Normal` (- (`KismetMathLibrary.MakeVector` _returnvalue_x _returnvalue_y (+ _returnvalue_z 200.0)) (`self.K2_GetActorLocation` _projectile))) (* (`self.ProjectileSpeed`) (`/Game/Blueprints/Enemies/Projectiles/BP_Projectile_Base.ThrowSpeedMultiplier` (`self.Projectile`)))) false "None")
      (`GameplayStatics.PlaySoundAtLocation` "/Game/Audio/SFX/Throw.Throw" (`self.K2_GetActorLocation` (`self.Projectile`)) (struct) 2.0 1.0 0.0 "/Game/Audio/IDKWhyIHaveToMakeThis.IDKWhyIHaveToMakeThis"))))

(fn `SmallThrowSeries`
  (set `self.WantsToThrow` 1))

(fn `SpawnProjectile`
  (params (AttachPoint :type "SceneComponent Object Reference") (Type :type "/Game/Blueprints/Enemies/Projectiles/BP_Projectile_Base Class Reference"))
  (bind _returnvalue (`|SpawnActorFromClass` Type (`KismetMathLibrary.MakeTransform` (0.0 0.0 0.0)) "Undefined" "OverrideRootScale"))
  (bind _output_get (set `self.Projectile` _returnvalue))
  (`self.K2_AttachToComponent` _output_get AttachPoint "None" "SnapToTarget" "SnapToTarget" "KeepWorld" true))

(fn `UserConstructionScript`
  (`parent.UserConstructionScript`))