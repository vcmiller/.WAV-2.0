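; Base enemy actor that tracks health, caches the player on spawn and destroys itself when health runs out.
; Attack, Swipe and StartPivot set request flags, which OnAttackBegin clears while opening the damage state and resetting the hit list.
; DealDamage uses that list to avoid repeat hits and skips fellow enemies.
; Taking damage triggers alert once, and a helper registers the enemy as a boss on the PlayerUI widget.
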(event `self.ReceiveBeginPlay`
  (set `self.Health` (`self.MaxHealth`))
  (bind _outactors (`GameplayStatics.GetAllActorsOfClass` "/Game/Blueprints/Player/BP_Player.BP_Player_C"))
  (set `self.Player` (`KismetArrayLibrary.Array_Get` _outactors)))

(event `DealDamage`
  (params (DamagedActor :type "Actor Object Reference") (Amount :type "Float (double-precision)"))
  (if (not (`BlueprintSetLibrary.Set_Contains` (`self.HitActors`) DamagedActor))
    (`BlueprintSetLibrary.Set_Add` (`self.HitActors`) DamagedActor)
    (if (`self.DoingDamage`)
      (cast `/Game/Blueprints/Enemies/BP_EnemyBase` DamagedActor
        (:`CastFailed`
          (`GameplayStatics.ApplyDamage` DamagedActor Amount null self))))))

(event `self.ReceiveAnyDamage`
  (params (Damage :type "Float (single-precision)") (DamageType :type "DamageType Object Reference") (InstigatedBy :type "Controller Object Reference") (DamageCauser :type "Actor Object Reference"))
  (`|ExecutionSequence`
    (:`then_0`
      (`/Engine/EditorBlueprintResources/StandardMacros.DoOnce` false
        (:`Completed`
          (set `self.Alerted` true))))
    (:`then_1`
      (bind _output_get (set `self.Health` (- (`self.Health`) Damage)))
      (`/Engine/EditorBlueprintResources/StandardMacros.CompareFloat` _output_get
        (:`==`
          _)
        (:`<`
          _))
      (`self.Die`))))

(fn `Alert`
  (set `self.Alerted` true)
  (`KismetSystemLibrary.PrintString` (`KismetSystemLibrary.GetDisplayName` self)))

(fn `Attack`
  (set `self.WantsToAttack` true))

(fn `DB_AddHealthBar`
  (bind _foundwidgets (`WidgetBlueprintLibrary.GetAllWidgetsOfClass` "/Game/UI/PlayerUI.PlayerUI_C"))
  (if (== (`KismetArrayLibrary.Array_Length` _foundwidgets) 0)
    (bind _returnvalue (`|CreateWidget` "/Game/UI/PlayerUI.PlayerUI_C" (`GameplayStatics.GetPlayerController` 0)))
    (`UserWidget.AddToViewport` _returnvalue 0)
    (`/Game/UI/PlayerUI.AddBoss` _returnvalue self)
    (else
      (`/Game/UI/PlayerUI.AddBoss` (`KismetArrayLibrary.Array_Get` _foundwidgets) self))))

(fn `Die`
  (`self.K2_DestroyActor`))

(fn `OnAttackBegin`
  (`BlueprintSetLibrary.Set_Clear` (`self.HitActors`))
  (set `self.WantsToAttack` false)
  (set `self.WantsToSwipe` false)
  (set `self.IsPivoting` false)
  (set `self.DoingDamage` true))

(fn `StartPivot`
  (set `self.IsPivoting` true))

(fn `Swipe`
  (set `self.WantsToSwipe` true))

(fn `UserConstructionScript`)