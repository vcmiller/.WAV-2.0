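; Player character with fixed-camera zones, camera-relative movement, running, jumping, cooldown-limited rolls and three melee attack inputs.
; Overlapped BP_CamZones feed a camera list whose last entry becomes the blended view target.
; Attack inputs queue a two-phase combo; functions swap weapon meshes, rate-limit turning, and toggle trails and once-per-actor hit damage.
; Lock-on is unfinished: it records nearby enemies' times but never assigns a target.
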(event `self.ReceiveTick`
  (params (DeltaSeconds :type "Float (single-precision)"))
  (`|ExecutionSequence`
    (:`then_0`
      (`self.CameraControl`
        (:`One Comes Out`
          (`self.UpdateRotation`)
          (bind _output_get (set `self.TimeUntilPhaseReset` (- (`self.TimeUntilPhaseReset`) DeltaSeconds)))
          (if (and (< _output_get 0.0) (not (`self.WantsToAttack`)))
            (set `self.AttackPhase` -1)))))
    (:`then_1`
      (set `self.CurrentRollCooldown` (- (`self.CurrentRollCooldown`) DeltaSeconds)))))

(event `self.ReceiveActorBeginOverlap`
  (params (OtherActor :type "Actor Object Reference"))
  ;[1 1 1] On Entering a New Camera Zone
  (bind _asbp_cam_zone (cast `/Game/Blueprints/Camera/BP_CamZone` OtherActor))
  (`KismetArrayLibrary.Array_AddUnique` (`self.CameraList`) (`/Game/Blueprints/Camera/BP_CamZone.CamActor` _asbp_cam_zone)))

(event `self.ReceiveActorEndOverlap`
  (params (OtherActor :type "Actor Object Reference"))
  ;[1 1 1] On Exiting a Camera Zone
  (bind _asbp_cam_zone (cast `/Game/Blueprints/Camera/BP_CamZone` OtherActor))
  (`KismetArrayLibrary.Array_RemoveItem` (`self.CameraList`) (`/Game/Blueprints/Camera/BP_CamZone.CamActor` _asbp_cam_zone)))

(event `self.ReceiveBeginPlay`
  (`PlayerController.SetViewTargetWithBlend` (`GameplayStatics.GetPlayerController` 0) (`KismetArrayLibrary.Array_Get` (`self.CameraList`)) 0.0 "VTBlend_Linear" 0.0 false)
  (bind _outactors (`GameplayStatics.GetAllActorsOfClass` "/Game/Blueprints/Camera/BP_CamZone.BP_CamZone_C"))
  (set `self.CamZoneList` _outactors)
  (bind _asbp_sword_trail (cast `/Game/Blueprints/BP_SwordTrail` (`ChildActorComponent.ChildActor` (`self.Trail`))))
  (bind _output_get (set `self.TrailObject` _asbp_sword_trail))
  (`SceneComponent.SetVisibility` (`/Game/Blueprints/BP_SwordTrail.Trail` _output_get) false false))

(event `InputAction|Jump`
  (params (Key :type "Key Structure" :default "AnyKey"))
  (:`Pressed`
    (if (not (`self.Attacking`))
      (`self.Jump`)))
  (:`Released`
    (`self.StopJumping`)))

(event `InputAxis|MoveForward`
  (params (AxisValue :type "Float (single-precision)"))
  (bind (_returnvalue_x _returnvalue_y) (`KismetMathLibrary.BreakVector` (`self.GetActorForwardVector` (`Controller.GetViewTarget` (`GameplayStatics.GetPlayerController` 0)))))
  (if (not (`self.Attacking`))
    (`self.AddMovementInput` (`KismetMathLibrary.Normal` (`KismetMathLibrary.MakeVector` _returnvalue_x _returnvalue_y)) AxisValue)))

(event `InputAxis|MoveRight`
  (params (AxisValue :type "Float (single-precision)"))
  (bind (_returnvalue_x _returnvalue_y) (`KismetMathLibrary.BreakVector` (`self.GetActorRightVector` (`Controller.GetViewTarget` (`GameplayStatics.GetPlayerController` 0)))))
  (if (not (`self.Attacking`))
    (`self.AddMovementInput` (`KismetMathLibrary.Normal` (`KismetMathLibrary.MakeVector` _returnvalue_x _returnvalue_y)) AxisValue)))

(event `InputAction|Attack1`
  (params (Key :type "Key Structure" :default "AnyKey"))
  ;[1 1 1] Attacks
  (:`Pressed`
    (`self.AttackInput` 0)))

(event `InputAction|Attack2`
  (params (Key :type "Key Structure" :default "AnyKey"))
  ;[1 1 1] Attacks
  (:`Pressed`
    (`self.AttackInput` 1)))

(event `InputAction|Attack3`
  (params (Key :type "Key Structure" :default "AnyKey"))
  ;[1 1 1] Attacks
  (:`Pressed`
    (`self.AttackInput` 2)))

(event `self.WeaponMesh.OnComponentBeginOverlap`
  (params (OverlappedComponent :type "PrimitiveComponent Object Reference") (OtherActor :type "Actor Object Reference") (OtherComp :type "PrimitiveComponent Object Reference") (OtherBodyIndex :type Integer) (bFromSweep :type Boolean) (SweepResult :type "HitResult Structure (by ref)"))
  (bind (_item_weaponmesh _item_phasereset _item_weaponscale _item_damage) (break `/Game/Blueprints/Structs/PlayerAttack` (`KismetArrayLibrary.Array_Get` (`self.Attacks`) (`self.PrevWeapon`))))
  (if (`self.Damaging`)
    (bind _returnvalue (`BlueprintSetLibrary.Set_Add` (`self.HitActors`) OtherActor))
    (if _returnvalue
      (`GameplayStatics.ApplyDamage` OtherActor _item_damage))))

(event `InputAction|Roll`
  (params (Key :type "Key Structure" :default "AnyKey"))
  (:`Pressed`
    (`self.K2_SetActorRotation` (`KismetMathLibrary.MakeRotFromZX` (0.0 0.0 1.0) (`self.GetLastMovementInputVector`)))
    (if (<= (`self.CurrentRollCooldown`) 0.0)
      (set `self.WantsToRoll` true))))

(event `InputAction|Run`
  (params (Key :type "Key Structure" :default "AnyKey"))
  (bind _charactermovement (`self.CharacterMovement`))
  (:`Pressed`
    (set `self.Running` true)
    (set `CharacterMovementComponent.MaxWalkSpeed` 1000.0 _charactermovement))
  (:`Released`
    (set `self.Running` false)
    (set `CharacterMovementComponent.MaxWalkSpeed` 500.0 _charactermovement)))

(event `InputAction|Lockon`
  (params (Key :type "Key Structure" :default "AnyKey"))
  (bind _lockonlasttime (`self.LockonLastTime`))
  (:`Pressed`
    (`/Engine/EditorBlueprintResources/StandardMacros.IsValid` (`self.LockonTarget`)
      (:`Is Valid`
        (set `self.LockonTarget` null))
      (:`Is Not Valid`
        (bind _outactors (`KismetSystemLibrary.SphereOverlapActors` (`self.K2_GetActorLocation`) 1500.0 (`|MakeArray` "ObjectTypeQuery3" :!type "EObjectTypeQuery Enum") "/Game/Blueprints/BP_EnemyBase.BP_EnemyBase_C"))
        ;[1 1 1] Find the least recently "locked-on" target
        (for _array_element _outactors
          (bind _asbp_enemy_base (cast `/Game/Blueprints/BP_EnemyBase` _array_element :!pure true))
          (if (`.ReturnValue` (`BlueprintMapLibrary.Map_Find` _lockonlasttime _asbp_enemy_base))
            (if true
              _)
            (else
              (`BlueprintMapLibrary.Map_Add` _lockonlasttime _asbp_enemy_base (`KismetSystemLibrary.GetGameTimeInSeconds`))
              (break))))))))

(fn `AttackInput`
  (params (Weapon :type Integer))
  (if (`KismetMathLibrary.BooleanNOR` (`NavMovementComponent.IsFalling` (`self.CharacterMovement`)) (`self.WantsToAttack`))
    (set `self.WantsToAttack` true)
    (set `self.Weapon` Weapon)
    (set `self.AttackPhase` (mod (+ (`self.AttackPhase`) 1) 2))))

(fn `BeginAttack`
  (params (Weapon :type Integer))
  (bind _weaponmesh (`self.WeaponMesh`))
  (bind (_item_weaponmesh _item_phasereset _item_weaponscale) (break `/Game/Blueprints/Structs/PlayerAttack` (`KismetArrayLibrary.Array_Get` (`self.Attacks`) Weapon)))
  (set `self.Attacking` true)
  (set `self.WantsToAttack` false)
  (set `self.TimeUntilPhaseReset` _item_phasereset)
  (`StaticMeshComponent.SetStaticMesh` _weaponmesh _item_weaponmesh)
  (`SceneComponent.SetRelativeScale3D` _weaponmesh (`KismetMathLibrary.MakeVector` _item_weaponscale _item_weaponscale _item_weaponscale))
  (if (!= (`self.PrevWeapon`) Weapon)
    (`ActorComponent.Activate` (`self.WeaponParticles`) true)
    (set `self.PrevWeapon` Weapon)))

(fn `BeginRoll`
  (`SceneComponent.SetVisibility` (`self.WeaponMesh`) false false))

(fn `EndDamage`
  (set `self.Damaging` false)
  (`SceneComponent.SetVisibility` (`/Game/Blueprints/BP_SwordTrail.Trail` (`self.TrailObject`)) false false))

(fn `EndRoll`
  (`SceneComponent.SetVisibility` (`self.WeaponMesh`) true false)
  (set `self.WantsToRoll` false)
  (set `self.CurrentRollCooldown` (`self.RollCooldown`)))

(fn `RotationDuringAttack`
  (bind _returnvalue (`self.GetActorForwardVector`))
  (bind (_returnvalue_roll _returnvalue_pitch _returnvalue_yaw) (`KismetMathLibrary.BreakRotator` (`self.K2_GetActorRotation`)))
  (bind _returnvalue_2 (`Controller.GetViewTarget` (`GameplayStatics.GetPlayerController` 0)))
  (bind (_returnvalue_x _returnvalue_y) (`KismetMathLibrary.BreakVector` (`self.GetActorForwardVector` _returnvalue_2)))
  (bind (_returnvalue_x_2 _returnvalue_y_2) (`KismetMathLibrary.BreakVector` (`self.GetActorRightVector` _returnvalue_2)))
  (bind _returnvalue_3 (`KismetMathLibrary.Normal` (+ (* (`KismetMathLibrary.Normal` (`KismetMathLibrary.MakeVector` _returnvalue_x _returnvalue_y)) (`self.GetInputAxisValue`)) (* (`KismetMathLibrary.Normal` (`KismetMathLibrary.MakeVector` _returnvalue_x_2 _returnvalue_y_2)) (`self.GetInputAxisValue`)))))
  (bind (_returnvalue_x_3 _returnvalue_y_3 _returnvalue_z) (`KismetMathLibrary.BreakVector` (`KismetMathLibrary.Cross_VectorVector` _returnvalue _returnvalue_3)))
  (`self.K2_SetActorRotation` (`KismetMathLibrary.MakeRotator` _returnvalue_roll _returnvalue_pitch (+ (* (`KismetMathLibrary.FClamp` (`KismetMathLibrary.DegAcos` (`KismetMathLibrary.Dot_VectorVector` _returnvalue _returnvalue_3)) 0.0 (* (`self.RotateSpeedAttacking`) (`GameplayStatics.GetWorldDeltaSeconds`))) (`KismetMathLibrary.SignOfFloat` _returnvalue_z)) _returnvalue_yaw))))

(fn `StartDamage`
  (bind _trailobject (`self.TrailObject`))
  (bind (_item_weaponmesh _item_phasereset _item_weaponscale _item_damage _item_trailpoint1 _item_trailpoint2) (break `/Game/Blueprints/Structs/PlayerAttack` (`KismetArrayLibrary.Array_Get` (`self.Attacks`) (`self.PrevWeapon`))))
  (`BlueprintSetLibrary.Set_Clear` (`self.HitActors`))
  (set `self.Damaging` true)
  (`SceneComponent.SetVisibility` (`/Game/Blueprints/BP_SwordTrail.Trail` (`self.TrailObject`)) true false)
  (set `/Game/Blueprints/BP_SwordTrail.Vertex2` _item_trailpoint2 _trailobject)
  (set `/Game/Blueprints/BP_SwordTrail.Vertex1` _item_trailpoint1 _trailobject))

(fn `UpdateRotation`
  (bind _attacking (`self.Attacking`))
  (set `CharacterMovementComponent.bOrientRotationToMovement` (not _attacking) (`self.CharacterMovement`))
  (if _attacking
    (`self.RotationDuringAttack`)))

(fn `UserConstructionScript`
  (bind _returnvalue (`self.K2_GetActorLocation` (`KismetArrayLibrary.Array_Get` (`self.CameraList`))))
  (bind _outactors (`KismetSystemLibrary.ComponentOverlapActors` (`self.CapsuleComponent`) (`self.GetTransform`) (`|MakeArray` "ObjectTypeQuery1" :!type "EObjectTypeQuery Enum") "/Game/Blueprints/Camera/BP_CamZone.BP_CamZone_C"))
  (for _array_element _outactors
    (bind _asbp_cam_zone (cast `/Game/Blueprints/Camera/BP_CamZone` _array_element))
    (`KismetArrayLibrary.Array_Set` (`self.CameraList`) 0 (`/Game/Blueprints/Camera/BP_CamZone.CamActor` _asbp_cam_zone))
    (break))
  (`KismetSystemLibrary.DrawDebugSphere` _returnvalue 100.0 12 (struct :`R` 0.94902 :`B` 1.0 :`A` 1.0) 0.2)
  (`KismetSystemLibrary.DrawDebugLine` _returnvalue (`self.K2_GetActorLocation`) (struct :`R` 0.94902 :`B` 1.0 :`A` 1.0) 0.2))