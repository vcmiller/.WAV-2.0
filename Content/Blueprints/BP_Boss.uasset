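; BP_Boss is a boss actor that registers itself with the player's UI when play begins.
; After running its parent's BeginPlay, it searches for a top-level PlayerUI widget and passes itself to AddBoss on the first one found.
; If none exists, it creates a PlayerUI for the first player controller, adds it to the viewport and registers there.
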(event `self.ReceiveBeginPlay`
  (`parent.ReceiveBeginPlay`)
  (bind _foundwidgets (`WidgetBlueprintLibrary.GetAllWidgetsOfClass` "/Game/UI/PlayerUI.PlayerUI_C"))
  (if (== (`KismetArrayLibrary.Array_Length` _foundwidgets) 0)
    (bind _returnvalue (`|CreateWidget` "/Game/UI/PlayerUI.PlayerUI_C" (`GameplayStatics.GetPlayerController` 0)))
    (`UserWidget.AddToViewport` _returnvalue 0)
    (`/Game/UI/PlayerUI.AddBoss` _returnvalue self)
    (else
      (`/Game/UI/PlayerUI.AddBoss` (`KismetArrayLibrary.Array_Get` _foundwidgets) self))))

(fn `UserConstructionScript`
  (`parent.UserConstructionScript`))