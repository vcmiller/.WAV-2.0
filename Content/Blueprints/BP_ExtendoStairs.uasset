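; BP_ExtendoStairs is an extendable staircase that unfolds from a vertical stack of steps into a flight positioned relative to Dest.
; The construction script rebuilds the stack from NumStairs, using separate end and middle meshes.
; Tick advances a clamped Extension value by OpenSpeed or CloseSpeed, depending on the Open flag.
; UpdateExtension gives each step its own slice of that value, so steps lerp into place sequentially, starting from the top.
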(event `self.ReceiveBeginPlay`)

(event `self.ReceiveTick`
  (params (DeltaSeconds :type "Float (single-precision)"))
  (set `self.Extension` (`KismetMathLibrary.FClamp` (+ (* DeltaSeconds (`KismetMathLibrary.SelectFloat` (`self.OpenSpeed`) (`self.CloseSpeed`) (`self.Open?`))) (`self.Extension`))))
  (`self.UpdateExtension`))

(fn `UpdateExtension`
  (locals (PerStair :type "Float (double-precision)"))
  (bind _perstair (`local.PerStair`))
  (set `local.PerStair` (/ 1.0 (`KismetMathLibrary.Conv_IntToDouble` (`self.NumStairs`))))
  (for (_array_element _array_index) (`self.Stairs`)
    (bind _returnvalue (* _array_index _perstair))
    (`SceneComponent.K2_SetWorldLocation` _array_element (`KismetMathLibrary.VLerp` (+ (`self.K2_GetActorLocation`) (`KismetMathLibrary.MakeVector` 0.0 0.0 (* (- (- (`self.NumStairs`) 1) _array_index) 20.0))) (`KismetMathLibrary.TransformLocation` (`SceneComponent.K2_GetComponentToWorld` (`self.Dest`)) (`KismetMathLibrary.MakeVector` 0.0 (* _array_index (`self.StepLength`)) (* _array_index (`self.StepHeight`)))) (`KismetMathLibrary.MapRangeClamped` (`self.Extension`) _returnvalue (+ _returnvalue _perstair) 0.0 1.0)) false false)))

(fn `UserConstructionScript`
  (bind _returnvalue (- (`self.NumStairs`) 1))
  (for _array_element (`self.Stairs`)
    (`ActorComponent.K2_DestroyComponent` _array_element))
  (for _index (range (+ _returnvalue 1))
    (bind _returnvalue_2 (- _returnvalue _index))
    (bind _returnvalue_3 (`AddComponent|NODE_AddStaticMeshComponent-0` :`RelativeTransform` (`KismetMathLibrary.MakeTransform` (`KismetMathLibrary.MakeVector` 0.0 0.0 (* _returnvalue_2 20.0)))))
    (`KismetArrayLibrary.Array_Add` (`self.Stairs`) _returnvalue_3)
    (`StaticMeshComponent.SetStaticMesh` _returnvalue_3 (select `bool` (or (== _returnvalue_2 0) (== _returnvalue_2 _returnvalue)) :`false` "/Game/StaticMesh/Environment/StairMid.StairMid" :`true` "/Game/StaticMesh/Environment/StairEnd.StairEnd" :!type "StaticMesh Object Reference"))))