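; Camera helper actor that tracks the player along a spline, as the closest point on that spline to the player.
; On BeginPlay it caches the first BP_Player found in the level.
; Each Tick it looks for a SplineComponent on its attach parent's owner and moves toward the closest point.
; A fixed-alpha lerp covers 70% of the remaining distance per frame, so smoothing depends on frame rate.
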(event `self.ReceiveBeginPlay`
  (bind _outactors (`GameplayStatics.GetAllActorsOfClass` "/Game/Blueprints/BP_Player.BP_Player_C"))
  (set `self.Player` (`KismetArrayLibrary.Array_Get` _outactors)))

(event `self.ReceiveTick`
  (params (DeltaSeconds :type "Float (single-precision)"))
  (bind _returnvalue (`SceneComponent.GetAttachParent` (`self.K2_GetRootComponent`)))
  (bind _returnvalue_2 (`self.GetComponentByClass` (`ActorComponent.GetOwner` _returnvalue) "/Script/Engine.SplineComponent"))
  (`/Engine/EditorBlueprintResources/StandardMacros.IsValid` _returnvalue
    (:`Is Valid`
      (`/Engine/EditorBlueprintResources/StandardMacros.IsValid` _returnvalue_2
        (:`Is Valid`
          (`self.K2_SetActorLocation` (`KismetMathLibrary.VLerp` (`SplineComponent.FindLocationClosestToWorldLocation` _returnvalue_2 (`self.K2_GetActorLocation` (`self.Player`)) "World") (`self.K2_GetActorLocation`) 0.3)))))))

(fn `UserConstructionScript`)