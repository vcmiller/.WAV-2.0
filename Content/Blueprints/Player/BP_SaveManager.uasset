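; Save manager that owns the BP_Save instance, restores persistent objects and places the player at the current checkpoint.
; BeginPlay loads the save slot, or creates and writes a new save, then runs Load.
; Load passes the save to every BP_PersistentObject, then teleports the player to the checkpoint reported by the first BP_Checkpoint found.
; Save only writes the held instance to its slot, without gathering object state.
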(event `Load`
  (bind _outactors (`GameplayStatics.GetAllActorsOfClass` "/Game/Blueprints/Environment/BP_PersistentObject.BP_PersistentObject_C"))
  (for _array_element _outactors
    (`/Game/Blueprints/Environment/BP_PersistentObject.Load` _array_element (`self.SaveGameInstance`)))
  (bind _outactors_2 (`GameplayStatics.GetAllActorsOfClass` "/Game/Blueprints/Environment/BP_Checkpoint.BP_Checkpoint_C"))
  (bind _out (`/Game/Blueprints/Environment/BP_Checkpoint.GetCurrentCheckpoint` (`KismetArrayLibrary.Array_Get` _outactors_2)))
  (`/Engine/EditorBlueprintResources/StandardMacros.IsValid` _out
    (:`Is Valid`
      (`self.K2_SetActorLocation` (`GameplayStatics.GetPlayerCharacter` 0) (`SceneComponent.K2_GetComponentLocation` (`/Game/Blueprints/Environment/BP_Checkpoint.SpawnPoint` _out)) false true))))

(event `Save`
  (bind _savegameinstance (`self.SaveGameInstance`))
  (`GameplayStatics.SaveGameToSlot` _savegameinstance (`/Game/Blueprints/Player/BP_Save.SlotName` _savegameinstance) (`/Game/Blueprints/Player/BP_Save.UserIndex` _savegameinstance)))

(event `self.ReceiveBeginPlay`
  (bind _returnvalue (`GameplayStatics.LoadGameFromSlot` (`self.SlotName`) (`self.UserIndex`)))
  (bind _asbp_save (cast `/Game/Blueprints/Player/BP_Save` _returnvalue)
    (:`then`
      (set `self.SaveGameInstance` _asbp_save)
      (`self.Load`))
    (:`CastFailed`
      (bind _returnvalue_2 (`GameplayStatics.CreateSaveGameObject` "/Game/Blueprints/Player/BP_Save.BP_Save_C"))
      (bind _output_get (set `self.SaveGameInstance` _returnvalue_2))
      (set `/Game/Blueprints/Player/BP_Save.SlotName` (`self.SlotName`) _output_get)
      (set `/Game/Blueprints/Player/BP_Save.UserIndex` (`self.UserIndex`) (`self.SaveGameInstance`))
      (`self.Save`)
      (`self.Load`))))

(fn `UserConstructionScript`)