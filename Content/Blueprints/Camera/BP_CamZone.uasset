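; BP_CamZone is a camera zone actor meant to blend the view to its CamActor when the player is involved, but that switch is currently disconnected.
; BeginPlay caches the first BP_Player found as Player.
; An unreachable branch compares OtherActor to Player and calls SetViewTargetWithBlend with a cubic blend over BlendTime.
; The overlap event, Tick and construction script do nothing.
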(event `self.ReceiveBeginPlay`
  (`|ExecutionSequence`
    (:`then_0`
      (bind _outactors (`GameplayStatics.GetAllActorsOfClass` "/Game/Blueprints/BP_Player.BP_Player_C"))
      (set `self.Player` (`KismetArrayLibrary.Array_Get` _outactors)))))

(event `self.ReceiveActorBeginOverlap`
  (params (OtherActor :type "Actor Object Reference")))

(fn `UserConstructionScript`)