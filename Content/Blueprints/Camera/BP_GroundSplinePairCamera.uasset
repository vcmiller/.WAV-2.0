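; Camera actor that moves its parent CameraRig_Rail in step with the player's progress along a separate ground rail spline.
; BeginPlay caches the first BP_Player and the rail it is attached to.
; Each Tick finds the ground spline key nearest the player, passes it through InputKeyToDistance and divides by spline length.
; The resulting ratio sets both rails' CurrentPositionOnRail, pairing ground path to camera path.
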(event `self.ReceiveBeginPlay`
  (bind _outactors (`GameplayStatics.GetAllActorsOfClass` "/Game/Blueprints/BP_Player.BP_Player_C"))
  (set `self.Player` (`KismetArrayLibrary.Array_Get` _outactors))
  (set `self.CameraRail` (cast `CameraRig_Rail` (`ActorComponent.GetOwner` (`SceneComponent.GetAttachParent` (`self.K2_GetRootComponent`))) :!pure true)))

(event `self.ReceiveTick`
  (params (DeltaSeconds :type "Float (single-precision)"))
  (bind _returnvalue (`self.GetComponentByClass` (`self.GroundRail`) "/Script/Engine.SplineComponent"))
  (`/Engine/EditorBlueprintResources/StandardMacros.IsValid` _returnvalue
    (:`Is Valid`
      (bind _output_get (set `CameraRig_Rail.CurrentPositionOnRail` (/ (`self.InputKeyToDistance` _returnvalue (`SplineComponent.FindInputKeyClosestToWorldLocation` _returnvalue (`self.K2_GetActorLocation` (`self.Player`)))) (`SplineComponent.GetSplineLength` _returnvalue)) (`self.CameraRail`)))
      (set `CameraRig_Rail.CurrentPositionOnRail` _output_get (`self.GroundRail`)))))

(fn `UserConstructionScript`)