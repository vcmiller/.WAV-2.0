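; BP_SwordTrail is an actor that draws a sword swing trail as a procedural mesh ribbon.
; BeginPlay builds a fixed vertex strip with triangles and UVs, then applies the trail material.
; Each tick shifts the world-space history back one pair and writes the actor location plus a point along its forward vector at the head.
; It then converts the points to local space and recreates the mesh section.
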(event `self.ReceiveTick`
  (params (DeltaSeconds :type "Float (single-precision)"))
  (`self.UpdatePreviousP`)
  (`ProceduralMeshComponent.CreateMeshSection_LinearColor` :`self` (`self.Trail`) :`Vertices` (`self.MapVertexArray`) :`Triangles` (`self.Triangles`) :`UV0` (`self.UVs`)))

(event `self.ReceiveBeginPlay`
  (bind _triangles (`self.Triangles`))
  (for _index (range 39)
    (`KismetArrayLibrary.Array_Add` _triangles (+ _index 0))
    (`KismetArrayLibrary.Array_Add` _triangles (+ _index 1))
    (`KismetArrayLibrary.Array_Add` _triangles (+ _index 2)))
  (for _ (range 40)
    (`KismetArrayLibrary.Array_Add` (`self.Vertices`) (0.0 0.0 0.0)))
  (for _index_2 (range 40)
    (`KismetArrayLibrary.Array_Add` (`self.UVs`) (`KismetMathLibrary.MakeVector2D` (/ (`KismetMathLibrary.Conv_IntToDouble` (/ _index_2 2)) 20.0) (`KismetMathLibrary.Conv_IntToDouble` (mod _index_2 2)))))
  (`ProceduralMeshComponent.CreateMeshSection_LinearColor` :`self` (`self.Trail`) :`Vertices` (`self.Vertices`) :`Triangles` (`self.Triangles`) :`UV0` (`self.UVs`) :`bCreateCollision` true)
  (set `self.Generated` true)
  (`self.UpdatePreviousP`)
  (`PrimitiveComponent.SetMaterial` (`self.Trail`) 0 "/Game/Materials/M_SwordTrail.M_SwordTrail"))

(fn `GetUpperVert`
  (returns (Out :type "Vector Structure"))
  (return (+ (`self.K2_GetActorLocation`) (* (`self.GetActorForwardVector`) 100.0))))

(fn `MapVertexArray`
  (returns (Out :type "Array of Vector Structure"))
  (bind _tempvertices (`self.TempVertices`))
  (`KismetArrayLibrary.Array_Clear` (`self.TempVertices`))
  (for _array_element (`self.Vertices`)
    (`KismetArrayLibrary.Array_Add` _tempvertices (`KismetMathLibrary.InverseTransformLocation` (`self.GetTransform`) _array_element)))
  (return _tempvertices))

(fn `Moved`)

(fn `UpdatePreviousP`
  (bind _vertices (`self.Vertices`))
  (bind _vertices_2 (`self.Vertices`))
  (bind _returnvalue (`KismetArrayLibrary.Array_LastIndex` (`self.Vertices`)))
  (for _index (range (+ (- _returnvalue 2) 1))
    (bind _returnvalue_2 (- _returnvalue _index))
    (`KismetArrayLibrary.Array_Set` _vertices_2 _returnvalue_2 (`KismetArrayLibrary.Array_Get` _vertices_2 (- _returnvalue_2 2))))
  (`KismetArrayLibrary.Array_Set` _vertices 0 (`self.K2_GetActorLocation`))
  (`KismetArrayLibrary.Array_Set` _vertices 1 (`self.GetUpperVert`)))

(fn `UserConstructionScript`)