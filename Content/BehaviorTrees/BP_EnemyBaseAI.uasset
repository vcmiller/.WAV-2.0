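; Base AI controller for enemy pawns that starts the behavior tree defined on the possessed BP_EnemyBase.
; On BeginPlay it caches the controlled enemy, initializes that enemy's Blackboard and runs its tree, stopping if the cast fails.
; An empty ConfigureBlackboard event, called before the tree runs, acts as a hook for blackboard setup.
; Helper functions switch to a new tree or stop the current brain logic.
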(event `self.ReceiveBeginPlay`
  (bind _asbp_enemy_base (cast `/Game/Blueprints/Enemies/BP_EnemyBase` (`self.K2_GetPawn`)))
  (bind _output_get (set `self.EnemyBase` _asbp_enemy_base))
  (bind _blackboardcomponent (`self.UseBlackboard` (`/Game/Blueprints/Enemies/BP_EnemyBase.Blackboard` _output_get)))
  (`self.ConfigureBlackboard` _blackboardcomponent _output_get)
  (`self.RunBehaviorTree` (`/Game/Blueprints/Enemies/BP_EnemyBase.BehaviorTree` _output_get)))

(event `ConfigureBlackboard`
  (params (Blackboard :type "BlackboardComponent Object Reference") (ControlledEnemy :type "/Game/Blueprints/Enemies/BP_EnemyBase Object Reference")))

(fn `StopBehaviorTree`
  (`BrainComponent.StopLogic` (`self.BrainComponent`) ""))

(fn `SwitchBehaviorTree`
  (params (NewBTree :type "BehaviorTree Object Reference"))
  (`BrainComponent.StopLogic` (`self.BrainComponent`) "TIME TO GO")
  (`self.RunBehaviorTree` NewBTree))

(fn `UserConstructionScript`)